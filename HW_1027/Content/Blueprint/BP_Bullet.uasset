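; BP_Bullet is a bullet actor that kills enemies on contact and removes itself after a set lifetime.
; Tick accumulates elapsed time and destroys the bullet once it reaches LifeTime.
; An actor overlap destroys any BP_Enemy it hits, while the bullet itself carries on until its timer expires.
; The graphs contain no movement logic.
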(event `self.ReceiveTick`
  (params (DeltaSeconds :type "Float (single-precision)"))
  ;[1 1 1] LifeTime
  (set `self.Elapse` (+ DeltaSeconds (`self.Elapse`)))
  (if (>= (`self.Elapse`) (`self.LifeTime`))
    (`self.K2_DestroyActor`)))

(event `self.ReceiveActorBeginOverlap`
  (params (OtherActor :type "Actor Object Reference"))
  ;[1 1 1] Kill Enemy
  (bind _asbp_enemy (cast `/Game/Blueprint/BP_Enemy` OtherActor))
  (`self.K2_DestroyActor` _asbp_enemy))

(fn `UserConstructionScript`)